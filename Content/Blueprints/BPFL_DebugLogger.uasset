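; Blueprint function library of debug helpers that print vector values to screen.
; Print2DVector and Print3DVector each take a vector and a name, convert the components to text, and format them into one labeled line.
; The result goes through PrintString with its other settings left at defaults.
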(fn `Print2DVector`
  (params (vector :type "Object.Vector2D Structure") (name :type String))
  (bind (_x _y) (`KismetMathLibrary.BreakVector2D` vector))
  (`KismetSystemLibrary.PrintString` null (`KismetTextLibrary.Conv_TextToString` (`|FormatText` "Name: {Name}  X={X} Y={Y}" (`KismetTextLibrary.Conv_StringToText` name) (`KismetTextLibrary.Conv_DoubleToText` _x "HalfToEven") (`KismetTextLibrary.Conv_DoubleToText` _y "HalfToEven")))))

(fn `Print3DVector`
  (params (vector :type "Object.Vector Structure") (name :type String))
  (`KismetSystemLibrary.PrintString` null (`KismetTextLibrary.Conv_TextToString` (`|FormatText` "Name: {Name}  X={X} Y={Y} Z={Z}" (`KismetTextLibrary.Conv_StringToText` name) (`KismetTextLibrary.Conv_DoubleToText` (.x vector) "HalfToEven") (`KismetTextLibrary.Conv_DoubleToText` (.y vector) "HalfToEven") (`KismetTextLibrary.Conv_DoubleToText` (.z vector) "HalfToEven")))))