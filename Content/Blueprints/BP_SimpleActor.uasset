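; BP_SimpleActor is a minimal actor that spawns an in-game UI actor at its own position when play begins.
; On BeginPlay it gets its location from GetIngameLocation, which also prints a debug string, and spawns BP_IngameUI there, even if colliding.
; It stores the spawned actor in UiLayer and passes itself to it through SetDelegate.
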(event `self.ReceiveBeginPlay`
  (bind _location (`self.getIngameLocation`))
  (bind _returnvalue (`|SpawnActorFromClass` "/Game/Blueprints/GUI/BP_IngameUI.BP_IngameUI_C" (`KismetMathLibrary.MakeTransform` _location) true))
  (set `self.uiLayer` _returnvalue)
  (`/Game/Blueprints/GUI/BP_IngameUI.SetDelegate` (`self.uiLayer`) self))

(fn `getIngameLocation`
  (returns (location :type "Object.Vector Structure"))
  (`KismetSystemLibrary.PrintString` "GetIngameLocation")
  (return (`self.K2_GetActorLocation` self)))

(fn `UserConstructionScript`)