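; BP_IngameUI is an actor that keeps an image widget and a text widget on screen at a projected in-game world location.
; It creates both widgets on BeginPlay, then every tick requests the location from the object passed to SetDelegate.
; That location is projected to screen space, offset to a viewport-centred origin and divided by viewport scale before positioning both widgets.
; Debug prints report the coordinates or a missing delegate.
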(event `self.ReceiveTick`
  (params (DeltaSeconds :type "Float (single-precision)"))
  (`self.UpdateFromLocation`))

(event `self.ReceiveBeginPlay`
  (`self.CreateUIWidgets`))

(fn `Convert3DTo2DCoords`
  (params (location :type "Object.Vector Structure"))
  (returns (position :type "Object.Vector2D Structure"))
  (bind _returnvalue (/ (- (`PlayerController.ProjectWorldLocationToScreen` (`GameplayStatics.GetPlayerController` 0) location) (* (`WidgetLayoutLibrary.GetViewportSize`) 0.5)) (`WidgetLayoutLibrary.GetViewportScale`)))
  (`/Game/Blueprints/BPFL_DebugLogger.Print3DVector` location "Location: ")
  (`/Game/Blueprints/BPFL_DebugLogger.Print2DVector` _returnvalue "Converted Position: ")
  (return _returnvalue))

(fn `CreateUIWidgets`
  (`|ExecutionSequence`
    (:`then_0`
      (bind _returnvalue (`|CreateWidget` "/Game/Blueprints/GUI/BPW_UIImage.BPW_UIImage_C"))
      (set `self.UIImageWIdget` _returnvalue)
      (`UserWidget.AddToViewport` (`self.UIImageWIdget`)))
    (:`then_1`
      (bind _returnvalue_2 (`|CreateWidget` "/Game/Blueprints/GUI/BPW_UIText.BPW_UIText_C"))
      (set `self.UITextWidget` _returnvalue_2)
      (`UserWidget.AddToViewport` (`self.UITextWidget`)))))

(fn `SetDelegate`
  (params (delegate :type "/Game/Blueprints/Interfaces/BPI_IngameUIDelegate Interface"))
  (set `self.ingameUIDelegate` delegate))

(fn `UpdateFromLocation`
  (bind _ingameuidelegate (`self.ingameUIDelegate`))
  (if (`KismetSystemLibrary.IsValid` _ingameuidelegate)
    (bind _location (message `/Game/Blueprints/Interfaces/BPI_IngameUIDelegate.getIngameLocation` _ingameuidelegate))
    (bind _position (`self.Convert3DTo2DCoords` _location))
    (`self.UpdateUIPosition` _position)
    (else
      (`KismetSystemLibrary.PrintString` "IngameUIDelegate is NULL"))))

(fn `UpdateUIPosition`
  (params (position :type "Object.Vector2D Structure"))
  (`/Game/Blueprints/GUI/BPW_UIImage.SetPosition` (`self.UIImageWIdget`) position)
  (`/Game/Blueprints/GUI/BPW_UIText.SetPosition` (`self.UITextWidget`) position))

(fn `UserConstructionScript`)